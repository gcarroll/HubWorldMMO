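; Player State Blueprint that owns the RiftInventory component, exposes it through GetInventoryComponent, and smoke-tests it on BeginPlay.
; On authority, it waits for inventory initialization, then adds a test item to the Backpack container found by gameplay tag and prints the result, or reports failure.
; On remote instances, it prints the container count after a fixed delay rather than waiting for initialization, as a debug check of client-side inventory state.
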(event Custom|InventoryInitialized
  (params (bSuccess :type Boolean))
  (bind _riftinventory (Variables|Default|GetRiftInventory))
  (if bSuccess
    (bind _returnvalue (Class|RiftInventoryComponent|AddItemtoContainer _riftinventory "/Game/BP/Inventory/Items/DA_Item_Test.DA_Item_Test" (Class|RiftInventoryComponent|GetContainerbyTag _riftinventory "(TagName=\"Rift.Container.Backpack\")") 1))
    (Development|PrintString (Utilities|String|Append "Rift: " (Guid|ToString(Guid) _returnvalue)))
    (else
      (Development|PrintString "Rift Inventory Not Initialized"))))

(event EventBeginPlay
  (bind _riftinventory (Variables|Default|GetRiftInventory))
  (Networking|SwitchHasAuthority
    (:Authority
      (Class|RiftInventoryComponent|WaitforInitialized _riftinventory (delegate Custom|InventoryInitialized)))
    (:Remote
      (Utilities|FlowControl|Delay 2.0)
      (Development|PrintString (Utilities|String|Append "Rift: " (Utilities|String|ToString(Integer) (Utilities|Array|Length (Class|RiftInventoryComponent|GetAllContainers _riftinventory))))))))

(event EventTick
  (params (DeltaSeconds :type Float%20%28single-precision%29)))

(fn ConstructionScript)

(fn GetInventoryComponent
  (return (Variables|Default|GetRiftInventory)))